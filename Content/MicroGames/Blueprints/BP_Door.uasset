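; Key-locked door for a micro game that swings open when the first-person player enters its collision volume holding a key.
; A dynamic emissive material on the light brightens on overlap, turning green with a key or red without, and resets on exit.
; A timeline lerps the door rotation by 90 degrees and sets an Opening flag while running, with no closing logic.
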(event OnComponentBeginOverlap(Collision)
  (params (OverlappedComponent :type Primitive%20Component%20Object%20Reference) (OtherActor :type Actor%20Object%20Reference) (OtherComp :type Primitive%20Component%20Object%20Reference) (OtherBodyIndex :type Integer) (bFromSweep :type Boolean) (SweepResult :type Hit%20Result%20Structure%20%28by%20ref%29))
  ;[1 0.4499 0.3197] Set Light Colour Based On Key
  (if (== OtherActor (Variables|Default|GetAs%20BP%20First%20Person%20Character))
    (Rendering|Material|SetScalarParameterValue (Variables|Default|GetDynamicMaterial) "Intensity" 1e+02 :!class /Script/Engine.MaterialInstanceDynamic)
    (if (Variables|/Game/FirstPerson/Blueprints/BP_FirstPersonCharacter.BP_FirstPersonCharacter_C|GetHasKey (Variables|Default|GetAs%20BP%20First%20Person%20Character))
      (Rendering|Material|SetVectorParameterValue (Variables|Default|GetDynamicMaterial) "Colour" "(R=0.000000,G=1.000000,B=0.335470,A=1.000000)" :!class /Script/Engine.MaterialInstanceDynamic)
      (bind _alpha (Timeline|Timeline Play)
        (:Update
          (Variables|Default|SetOpening true)
          (Transformation|SetRelativeRotation (Variables|Default|GetSM_Door) (Math|Rotator|Lerp(Rotator) "0, 0, 0" "0.000000,90.000000,0.000000" _alpha) false false))
        (:Finished
          (Variables|Default|SetOpening false)))
      (else
        (Rendering|Material|SetVectorParameterValue (Variables|Default|GetDynamicMaterial) "Colour" "(R=1.000000,G=0.000000,B=0.000000,A=1.000000)" :!class /Script/Engine.MaterialInstanceDynamic)))))

(event OnComponentEndOverlap(Collision)
  (params (OverlappedComponent :type Primitive%20Component%20Object%20Reference) (OtherActor :type Actor%20Object%20Reference) (OtherComp :type Primitive%20Component%20Object%20Reference) (OtherBodyIndex :type Integer))
  ;[0.5869 1 0.6123] Return Light to Default
  (if (== OtherActor (Variables|Default|GetAs%20BP%20First%20Person%20Character))
    (Rendering|Material|SetScalarParameterValue (Variables|Default|GetDynamicMaterial) "Intensity" 1.0 :!class /Script/Engine.MaterialInstanceDynamic)
    (Rendering|Material|SetVectorParameterValue (Variables|Default|GetDynamicMaterial) "Colour" "(R=1.000000,G=0.760945,B=0.354083,A=1.000000)" :!class /Script/Engine.MaterialInstanceDynamic)))

(event EventBeginPlay
  ;[1 0.6236 0.714] Setup
  (bind _asbp_first_person_character (Utilities|Casting|CastToBP_FirstPersonCharacter (Game|GetPlayerCharacter 0)))
  (Variables|Default|SetAs%20BP%20First%20Person%20Character _asbp_first_person_character)
  (bind _returnvalue (Rendering|Material|CreateDynamicMaterialInstance "/Game/MicroGames/Materials/MI_Emission_Default.MI_Emission_Default" "None" "None" :!class /Script/Engine.KismetMaterialLibrary))
  (Variables|Default|SetDynamicMaterial _returnvalue)
  (Rendering|Material|SetMaterial (Variables|Default|GetLight) 0 (Variables|Default|GetDynamicMaterial)))

(fn ConstructionScript)