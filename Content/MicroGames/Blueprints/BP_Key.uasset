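; BP_Key is a key pickup that stays hidden and non-collidable until no BP_MovingTarget actors remain in the level.
; Tick polls the target count, using the index returned by an array Add, to toggle visibility and collision, firing a one-time explosion and sound on reveal.
; When the player's cached BP_FirstPersonCharacter overlaps the revealed key, it sets HasKey, plays a sound and destroys itself.
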(event OnComponentBeginOverlap(Collision)
  (params (OverlappedComponent :type Primitive%20Component%20Object%20Reference) (OtherActor :type Actor%20Object%20Reference) (OtherComp :type Primitive%20Component%20Object%20Reference) (OtherBodyIndex :type Integer) (bFromSweep :type Boolean) (SweepResult :type Hit%20Result%20Structure%20%28by%20ref%29))
  ;[1 1 1] Collecting the Key
  (if (and (== OtherActor (Variables|Default|GetAs%20BP%20First%20Person%20Character)) (Variables|Default|GetAllTargetsDestroyed))
    (Variables|/Game/FirstPerson/Blueprints/BP_FirstPersonCharacter.BP_FirstPersonCharacter_C|SetHasKey (Variables|Default|GetAs%20BP%20First%20Person%20Character) true)
    (Audio|PlaySoundatLocation "/Game/StarterContent/Audio/Fire01.Fire01" (Transformation|GetActorLocation) "0, 0, 0" 1.0 1.0 0.0 0 0 0 0)
    (Actor|DestroyActor)))

(event EventBeginPlay
  ;[1 1 1] Setup
  (bind _asbp_first_person_character (Utilities|Casting|CastToBP_FirstPersonCharacter (Game|GetPlayerCharacter 0)))
  (Variables|Default|SetAs%20BP%20First%20Person%20Character _asbp_first_person_character))

(event EventTick
  (params (DeltaSeconds :type Float%20%28single-precision%29))
  (bind _returnvalue (Transformation|GetActorLocation))
  ;[1 0.3524 0.4725] Key Visibility
  (bind _outactors (Actor|GetAllActorsOfClass "/Game/MicroGames/Blueprints/BP_MovingTarget.BP_MovingTarget_C"))
  (bind _returnvalue_2 (Utilities|Array|Add _outactors 0))
  (bind _output_get (Variables|Default|SetAllTargetsDestroyed (<= _returnvalue_2 0)))
  (Rendering|SetVisibility (Variables|Default|GetSM_Key) _output_get true)
  (Collision|SetActorEnableCollision _output_get)
  ;[1 1 1] Effects
  (if (Variables|Default|GetAllTargetsDestroyed)
    (Utilities|FlowControl|DoOnce false
      (:Completed
        (Effects|SpawnEmitteratLocation "/Game/StarterContent/Particles/P_Explosion.P_Explosion" _returnvalue)
        (Audio|PlaySoundatLocation "/Game/StarterContent/Audio/Collapse01.Collapse01" _returnvalue "0, 0, 0" 1.0 1.0 0.0 0 0 0 0)))))

(fn ConstructionScript)